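; Lobby player controller that tracks a player's character choice in a multiplayer game and passes it to GM_GameMode.
; AssignSelectedCharacter stores the ID and image, then CharacterCheck looks up the class in the game mode's Characters array.
; AssignPlayer writes both into PlayerSettings, and CallUpdate, also run by InitialSetup, calls SelectCharacter on the game mode.
; SetupLobbyMenu has an empty body.
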(event Custom|InitialSetup
  ;[1 1 1] Initial Setup
  (CallFunction|CallUpdate (Variables|Default|GetPlayer%20Settings)))

(event Custom|SetupLobbyMenu
  (params (ServerName :type Text)))

(event Custom|AssignPlayer
  (params (Character :type Character%20Class%20Reference) (CharacterImage :type Texture%202D%20Object%20Reference))
  (bind _player_settings (Variables|Default|GetPlayer%20Settings))
  ;[1 1 1] Assigns selected character
  (Utilities|Struct|SetmembersinSTRUCT_PlayerInfo _player_settings Character CharacterImage)
  (CallFunction|CallUpdate _player_settings))

(event Custom|CallUpdate
  (params (PlayerInfo :type STRUCT%20Player%20Info%20Structure))
  ;[1 1 1] Select Character + Update Everyone
  (Variables|Default|SetPlayer%20Settings PlayerInfo)
  (Default|SelectCharacter (.AsGM%20Game%20Mode (Utilities|Casting|CastToGM_GameMode (Game|GetGameMode))) self (.PlayerCharacter (Utilities|Struct|BreakSTRUCT_PlayerInfo (Variables|Default|GetPlayer%20Settings)))))

(event Custom|AssignSelectedCharacter
  (params (CharacterID :type Integer) (Character%20Image :type Texture%202D%20Object%20Reference))
  ;[1 1 1] Assign The Selected Character
  (Variables|Default|SetPrevious%20Selection (Variables|Default|GetSelected%20Character))
  (Variables|Default|SetCharacter%20Image Character%20Image)
  (Variables|Default|SetSelected%20Character CharacterID)
  (CallFunction|CharacterCheck))

(fn ConstructionScript)

(fn CharacterCheck
  (CallFunction|AssignPlayer (Utilities|Array|Get(acopy) (Variables|/Game/Multiplayer/LobbyContent/GM_GameMode.GM_GameMode_C|GetCharacters (.AsGM%20Game%20Mode (Utilities|Casting|CastToGM_GameMode (Game|GetGameMode)))) (Variables|Default|GetSelected%20Character)) (Variables|Default|GetCharacter%20Image)))

(fn LobbyPCRef
  (return self))