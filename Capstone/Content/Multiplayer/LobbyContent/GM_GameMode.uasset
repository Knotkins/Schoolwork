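; Multiplayer lobby game mode that registers joining players and spawns their selected characters.
; PostLogin records the player, caches PlayerStarts, reads server name and player limit from the game instance, then triggers the lobby controller's setup and menu.
; Game instance and controller are reached through message calls.
; SelectCharacter spawns the given class at a random PlayerStart's location, always using the first one's rotation, then possesses it.
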(event Custom|SelectCharacter
  (params (PlayerController :type Player%20Controller%20Object%20Reference) (Character%20Class :type Character%20Class%20Reference))
  (bind _spawnpoints (Variables|Default|GetSpawnPoints))
  ;[1 1 1] Spawn Selected Character
  (bind _returnvalue (Game|SpawnActorfromClass Character%20Class (Math|Transform|MakeTransform (Transformation|GetActorLocation (Utilities|Array|Get(acopy) _spawnpoints (Math|Random|RandomIntegerinRange 0 (- (Utilities|Array|Length _spawnpoints) 1)))) (Transformation|GetActorRotation (Utilities|Array|Get(acopy) _spawnpoints))) "AlwaysSpawn" 0 0))
  (Pawn|Possess PlayerController _returnvalue))

(event EventPostLogin
  (params (NewPlayer :type Player%20Controller%20Object%20Reference))
  ;[1 1 1] Handles Lobby Setup
  (bind _output_get (Variables|Default|SetConnectedPlayer NewPlayer))
  (Utilities|Array|AddUnique (Variables|Default|GetPlayers) _output_get)
  (bind _outactors (Actor|GetAllActorsOfClass "/Script/Engine.PlayerStart"))
  (Variables|Default|SetSpawnPoints _outactors)
  (bind _gameinstance (Class|BPIGameInstance|GameInstanceRef(Message) (Game|GetGameInstance)))
  (Variables|Default|SetServerName (Variables|/Game/Multiplayer/LobbyContent/BP_GameInstance.BP_GameInstance_C|GetServerName _gameinstance))
  (Variables|Default|SetMaxPlayers (Variables|/Game/Multiplayer/LobbyContent/BP_GameInstance.BP_GameInstance_C|GetMax#ofPlayers _gameinstance))
  (bind _pc (Class|PCIPlayerController|LobbyPCRef(Message) (Variables|Default|GetConnectedPlayer)))
  (Default|InitialSetup _pc)
  (Default|SetupLobbyMenu _pc (Variables|Default|GetServerName)))

(fn ConstructionScript)

(fn GameInstanceRef
  (return 0))