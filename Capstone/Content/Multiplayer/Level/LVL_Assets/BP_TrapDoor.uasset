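; BP_TrapDoor is a two-leaf trap door that a player opens by pressing F.
; Overlaps of Box by a BP_BaseCharacter enable and disable input for player controller 0, regardless of which character overlaps.
; F destroys Box and Box1, then snaps both closed door components to their open counterparts' relative transforms.
; The opening is one-way, with no interpolation or replication logic in the graph.
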(event OnComponentBeginOverlap(Box)
  (params (OverlappedComponent :type Primitive%20Component%20Object%20Reference) (OtherActor :type Actor%20Object%20Reference) (OtherComp :type Primitive%20Component%20Object%20Reference) (OtherBodyIndex :type Integer) (bFromSweep :type Boolean) (SweepResult :type Hit%20Result%20Structure%20%28by%20ref%29))
  (Utilities|Casting|CastToBP_BaseCharacter OtherActor)
  (Input|EnableInput (Game|GetPlayerController 0)))

(event OnComponentEndOverlap(Box)
  (params (OverlappedComponent :type Primitive%20Component%20Object%20Reference) (OtherActor :type Actor%20Object%20Reference) (OtherComp :type Primitive%20Component%20Object%20Reference) (OtherBodyIndex :type Integer))
  (Utilities|Casting|CastToBP_BaseCharacter OtherActor)
  (Input|DisableInput (Game|GetPlayerController 0)))

(event Input|KeyboardEvents|F
  (params (Key :type Key%20Structure))
  (bind _door1_open (Variables|Default|GetDoor1_Open))
  (bind _door2_open (Variables|Default|GetDoor2_Open))
  (:Pressed
    (Components|DestroyComponent (Variables|Default|GetBox))
    (Components|DestroyComponent (Variables|Default|GetBox1))
    (Transformation|SetRelativeLocationAndRotation (Variables|Default|GetDoor1_Closed) (Variables|/Script/Engine.SceneComponent|GetRelativeLocation _door1_open) (Variables|/Script/Engine.SceneComponent|GetRelativeRotation _door1_open) false false)
    (Transformation|SetRelativeLocationAndRotation (Variables|Default|GetDoor2_Closed) (Variables|/Script/Engine.SceneComponent|GetRelativeLocation _door2_open) (Variables|/Script/Engine.SceneComponent|GetRelativeRotation _door2_open) false false)))

(fn ConstructionScript)