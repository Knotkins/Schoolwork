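; BP_Door is a key-locked double door that a BP_BaseCharacter opens by interacting with it.
; Overlapping the Box shows a prompt widget, and sets AtDoor if the character's boolean Keys array is true at the door's KeyValue index.
; Leaving hides the widget and clears AtDoor.
; Interacting while AtDoor is set destroys the Box and snaps both door components to their open counterparts' relative transforms, with no closing logic.
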(event OnComponentBeginOverlap(Box)
  (params (OverlappedComponent :type Primitive%20Component%20Object%20Reference) (OtherActor :type Actor%20Object%20Reference) (OtherComp :type Primitive%20Component%20Object%20Reference) (OtherBodyIndex :type Integer) (bFromSweep :type Boolean) (SweepResult :type Hit%20Result%20Structure%20%28by%20ref%29))
  (Development|SetHiddeninGame (Variables|Default|GetWidget) false false)
  (bind _asbp_base_character (Utilities|Casting|CastToBP_BaseCharacter OtherActor))
  (for (_array_element _array_index) (Variables|/Game/Multiplayer/Characters/BP_BaseCharacter.BP_BaseCharacter_C|GetKeys _asbp_base_character)
    (if (and _array_element (== _array_index (Variables|Default|GetKeyValue)))
      (Variables|Default|SetAtDoor true))))

(event OnComponentEndOverlap(Box)
  (params (OverlappedComponent :type Primitive%20Component%20Object%20Reference) (OtherActor :type Actor%20Object%20Reference) (OtherComp :type Primitive%20Component%20Object%20Reference) (OtherBodyIndex :type Integer))
  (Development|SetHiddeninGame (Variables|Default|GetWidget) true false)
  (Utilities|Casting|CastToBP_BaseCharacter OtherActor)
  (Variables|Default|SetAtDoor false))

(event Custom|Open%20Door
  (bind _door1_open (Variables|Default|GetDoor1_Open))
  (bind _door2_open (Variables|Default|GetDoor2_Open))
  (Components|DestroyComponent (Variables|Default|GetBox))
  (Transformation|SetRelativeLocationAndRotation (Variables|Default|GetDoor1_Closed) (Variables|/Script/Engine.SceneComponent|GetRelativeLocation _door1_open) (Variables|/Script/Engine.SceneComponent|GetRelativeRotation _door1_open) false false)
  (Transformation|SetRelativeLocationAndRotation (Variables|Default|GetDoor2_Closed) (Variables|/Script/Engine.SceneComponent|GetRelativeLocation _door2_open) (Variables|/Script/Engine.SceneComponent|GetRelativeRotation _door2_open) false false))

(event EventInteracted
  (params (Interactor :type Pawn%20Object%20Reference))
  (Utilities|Casting|CastToBP_BaseCharacter Interactor)
  (if (Variables|Default|GetAtDoor)
    (CallFunction|OpenDoor)))

(fn ConstructionScript)