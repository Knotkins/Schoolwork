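; Key-locked double door that the player opens with F.
; Box overlap loops the character's Keys array, enabling input where the entry at KeyValue is true and setting "Door is locked" speech for every other entry, even when the key is held.
; Leaving the box disables input and clears the speech.
; F destroys the box and snaps both closed door components to their open counterparts' relative transforms, with no animation.
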(event OnComponentBeginOverlap(Box)
  (params (OverlappedComponent :type Primitive%20Component%20Object%20Reference) (OtherActor :type Actor%20Object%20Reference) (OtherComp :type Primitive%20Component%20Object%20Reference) (OtherBodyIndex :type Integer) (bFromSweep :type Boolean) (SweepResult :type Hit%20Result%20Structure%20%28by%20ref%29))
  (bind _asbp_base_character (Utilities|Casting|CastToBP_BaseCharacter OtherActor))
  (for (_array_element _array_index) (Variables|/Game/Multiplayer/Characters/BP_BaseCharacter.BP_BaseCharacter_C|GetKeys _asbp_base_character)
    (if (and _array_element (== _array_index (Variables|Default|GetKeyValue)))
      (Input|EnableInput (Game|GetPlayerController 0))
      (else
        (bind _asbp_base_character_2 (Utilities|Casting|CastToBP_BaseCharacter OtherActor))
        (Variables|/Game/Multiplayer/Characters/BP_BaseCharacter.BP_BaseCharacter_C|SetCharacter%20Speech _asbp_base_character_2 "Door is locked")))))

(event OnComponentEndOverlap(Box)
  (params (OverlappedComponent :type Primitive%20Component%20Object%20Reference) (OtherActor :type Actor%20Object%20Reference) (OtherComp :type Primitive%20Component%20Object%20Reference) (OtherBodyIndex :type Integer))
  (Utilities|Casting|CastToBP_BaseCharacter OtherActor)
  (Input|DisableInput (Game|GetPlayerController 0))
  (bind _asbp_base_character (Utilities|Casting|CastToBP_BaseCharacter OtherActor))
  (Variables|/Game/Multiplayer/Characters/BP_BaseCharacter.BP_BaseCharacter_C|SetCharacter%20Speech _asbp_base_character ""))

(event Input|KeyboardEvents|F
  (params (Key :type Key%20Structure))
  (bind _door1_open (Variables|Default|GetDoor1_Open))
  (bind _door2_open (Variables|Default|GetDoor2_Open))
  (:Pressed
    (Components|DestroyComponent (Variables|Default|GetBox))
    (Transformation|SetRelativeLocationAndRotation (Variables|Default|GetDoor1_Closed) (Variables|/Script/Engine.SceneComponent|GetRelativeLocation _door1_open) (Variables|/Script/Engine.SceneComponent|GetRelativeRotation _door1_open) false false)
    (Transformation|SetRelativeLocationAndRotation (Variables|Default|GetDoor2_Closed) (Variables|/Script/Engine.SceneComponent|GetRelativeLocation _door2_open) (Variables|/Script/Engine.SceneComponent|GetRelativeRotation _door2_open) false false)))

(fn ConstructionScript)