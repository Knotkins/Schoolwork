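; BP_Grid is a world-placed tile grid that maps terrain costs and pathfinds between the selected tile and the hovered tile.
; Sphere traces sample each cell for ground and BP_Base_Obstacle types, filling a coordinate-keyed tile map.
; Construction draws debug planes coloured by ground type, and BeginPlay spawns BP_GridTIle actors on non-empty cells.
; Hover changes run four-way A* with Manhattan heuristic and weighted tile costs, storing the retraced Path.
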(event Custom|Event_NewTileSelected
  (params (selectedTile :type BP%20Grid%20T%20Ile%20Object%20Reference))
  (Utilities|IsValid (Variables|Grid|GetselectedTile)
    (:Is%20Valid
      (Default|EventDeselectTIle (Variables|Grid|GetselectedTile)))
    (:Is%20Not%20Valid
      _))
  (Variables|Grid|SetselectedTile selectedTile))

(event Custom|Event_NewTileOvered
  (params (OveredTile :type BP%20Grid%20T%20Ile%20Object%20Reference))
  (bind _selectedtile (Variables|Grid|GetselectedTile))
  (Utilities|IsValid (Variables|Grid|GetoveredTile)
    (:Is%20Valid
      (Default|EventEndOverTile (Variables|Grid|GetoveredTile)))
    (:Is%20Not%20Valid
      _))
  (Variables|Grid|SetoveredTile OveredTile)
  (CallFunction|HighlightCurrentPath false)
  (if (and (Utilities|IsValid _selectedtile) (Utilities|IsValid (Variables|Grid|GetoveredTile)))
    (Pathfinding|FindPathtoTarget (Variables|/Game/Blueprints/Grids/BP_GridTIle.BP_GridTIle_C|GetgridIndex _selectedtile) (Variables|/Game/Blueprints/Grids/BP_GridTIle.BP_GridTIle_C|GetgridIndex (Variables|Grid|GetoveredTile)))
    (CallFunction|HighlightCurrentPath false)))

(event EventBeginPlay
  (Rendering|Debug|FlushPersistentDebugLines)
  (Variables|Grid|SetGridLocation (Transformation|GetWorldLocation (Variables|Default|GetScene)))
  (Grid|GenerateMapDatafromWorld)
  (Grid|SpawnTile false))

(fn ConstructionScript
  (bind _gridsizeworld (Variables|Grid|GetGridSizeWorld))
  (Rendering|Debug|FlushPersistentDebugLines)
  (bind _output_get (Variables|Grid|SetGridLocation (Transformation|GetWorldLocation (Variables|Default|GetScene))))
  (Rendering|Debug|DrawDebugBox _output_get (Math|Vector|MakeVector (.y _gridsizeworld) (.x _gridsizeworld) 5.0) (Variables|Debug|GetGridBoxColour) "0,0.000000, 0" 1e+09 1e+01)
  (Rendering|Debug|DrawDebugBox (Grid|GridBottemLeft) (Math|Vector|MakeVector 2e+01 2e+01 2e+01) (Variables|Debug|GetBottomLeftColour) "0, 0, 0" 1e+09 1e+01)
  (Grid|GenerateMapDatafromWorld)
  (Debug|DrawTile))

(fn GridBottemLeft
  (return (- (- (Variables|Grid|GetGridLocation) (* (Math|Vector|GetRightVector (Variables|Default|GetScene)) (.x (Variables|Grid|GetGridSizeWorld)))) (* (Math|Vector|GetForwardVector (Variables|Default|GetScene)) (.y (Variables|Grid|GetGridSizeWorld))))))

(fn GridTileNumber
  (bind _gridsizeworld (Variables|Grid|GetGridSizeWorld))
  (bind _tilesize (Variables|Grid|GetTileSize))
  (bind _returnvalue (/ _gridsizeworld _tilesize))
  (return (- (Math|Float|Round (.x _returnvalue)) 1) (- (Math|Float|Round (.y _returnvalue)) 1) 0))

(fn DrawTile
  (bind _keys (Utilities|Map|Keys (Variables|Grid|Getstruct_Tile)))
  (for _array_element _keys
    (Debug|MyDrawDebugPlane (.worldlocation (.Value (Utilities|Map|Find (Variables|Grid|Getstruct_Tile) _array_element))) (.groundtype (.Value (Utilities|Map|Find (Variables|Grid|Getstruct_Tile) _array_element))))))

(fn MySphereTrace
  (params (A :type Vector) (InputPin :type Vector) (TraceChannel :type ETraceTypeQuery%20Enum :default "TraceTypeQuery1"))
  (bind (_outhit _returnvalue) (Collision|SphereTraceByChannel (+ A "0.010000, 0, 0") InputPin (- (Variables|Grid|GetTileSize) (Variables|Grid|GetTileSizeMinus)) TraceChannel false 0 "None" true "(R=1.000000,G=0.000000,B=0.000000,A=1.000000)" "(R=0.000000,G=1.000000,B=0.000000,A=1.000000)" 2e+01))
  (return _returnvalue (.hitactor _outhit)))

(fn MyDrawDebugPlane
  (params (Location :type Vector) (GroundType :type Enum_GroundTypes%20Enum :default "NewEnumerator0"))
  (switch Utilities|FlowControl|Switch|SwitchonEnum_GroundTypes GroundType
    (:NewEnumerator0
      (LocalVariables|SetTileColour "(R=0.000000,G=1.000000,B=0.085310,A=1.000000)"))
    (:NewEnumerator1
      (LocalVariables|SetTileColour "(R=0.869792,G=0.855820,B=0.000000,A=1.000000)"))
    (:NewEnumerator2
      (LocalVariables|SetTileColour "(R=0.817708,G=0.275223,B=0.001199,A=1.000000)"))
    (:NewEnumerator3
      (LocalVariables|SetTileColour "(R=0.598958,G=0.000000,B=0.000000,A=1.000000)")))
  (Class|KismetSystemLibrary|DrawDebugPlane (Utilities|Struct|MakePlane (.Z (Math|Vector|BreakVector Location)) 0.0 0.0 1.0) Location (- (Variables|Grid|GetTileSize) (Variables|Grid|GetTileSizeMinus)) (LocalVariables|GetTileColour) 1e+04))

(fn GenerateMapDatafromWorld
  (bind (_gridtilenumberx _gridtilenumbery) (Grid|GridTileNumber))
  (bind _tilesize (Variables|Grid|GetTileSize))
  (bind _tilesize_2 (Variables|Grid|GetTileSize))
  (for _index (range 0 _gridtilenumberx)
    (LocalVariables|SetX _index)
    (for _index_2 (range 0 _gridtilenumbery)
      (LocalVariables|SetY _index_2)
      (LocalVariables|SetTilePostion (+ (Grid|GridBottemLeft) (* (Math|Vector|GetRightVector (Variables|Default|GetScene)) (+ (* (LocalVariables|GetX) (* _tilesize_2 2.0)) _tilesize_2)) (* (Math|Vector|GetForwardVector (Variables|Default|GetScene)) (+ (* (LocalVariables|GetY) (* _tilesize 2.0)) _tilesize))))
      (if (.HitSomething (Grid|MySphereTrace (LocalVariables|GetTilePostion) (LocalVariables|GetTilePostion) "TraceTypeQuery3"))
        (if (.HitSomething (Grid|MySphereTrace (LocalVariables|GetTilePostion) (LocalVariables|GetTilePostion) "TraceTypeQuery4"))
          (Utilities|Map|Add (Variables|Grid|Getstruct_Tile) (Math|Vector2D|MakeVector2D (Math|Conversions|ToFloat(Integer) (LocalVariables|GetX)) (Math|Conversions|ToFloat(Integer) (LocalVariables|GetY))) (Utilities|Struct|MakeStruct_Tiles 0 (Variables|/Game/Blueprints/Grids/BP_Base_Obstacle.BP_Base_Obstacle_C|GetEnum_GroundType (.AsBP%20Base%20Obstacle (Utilities|Casting|CastToBP_Base_Obstacle (.Actor (Grid|MySphereTrace (LocalVariables|GetTilePostion) (LocalVariables|GetTilePostion) "TraceTypeQuery4"))))) (LocalVariables|GetTilePostion) (Math|Vector2D|MakeVector2D (Math|Conversions|ToFloat(Integer) (LocalVariables|GetX)) (Math|Conversions|ToFloat(Integer) (LocalVariables|GetY))) (Grid|GetTileCost (Variables|/Game/Blueprints/Grids/BP_Base_Obstacle.BP_Base_Obstacle_C|GetEnum_GroundType (.AsBP%20Base%20Obstacle (Utilities|Casting|CastToBP_Base_Obstacle (.Actor (Grid|MySphereTrace (LocalVariables|GetTilePostion) (LocalVariables|GetTilePostion) "TraceTypeQuery4")))))) 0 0 0 "(X=0.000000,Y=0.000000)"))
          (else
            (Utilities|Map|Add (Variables|Grid|Getstruct_Tile) (Math|Vector2D|MakeVector2D (Math|Conversions|ToFloat(Integer) (LocalVariables|GetX)) (Math|Conversions|ToFloat(Integer) (LocalVariables|GetY))) (Utilities|Struct|MakeStruct_Tiles 0 "NewEnumerator0" (LocalVariables|GetTilePostion) (Math|Vector2D|MakeVector2D (Math|Conversions|ToFloat(Integer) (LocalVariables|GetX)) (Math|Conversions|ToFloat(Integer) (LocalVariables|GetY))) (Grid|GetTileCost "NewEnumerator0") 0 0 0 "(X=0.000000,Y=0.000000)"))))
        (else
          (Utilities|Map|Add (Variables|Grid|Getstruct_Tile) (Math|Vector2D|MakeVector2D (Math|Conversions|ToFloat(Integer) (LocalVariables|GetX)) (Math|Conversions|ToFloat(Integer) (LocalVariables|GetY))) (Utilities|Struct|MakeStruct_Tiles 0 "NewEnumerator4" (LocalVariables|GetTilePostion) (Math|Vector2D|MakeVector2D (Math|Conversions|ToFloat(Integer) (LocalVariables|GetX)) (Math|Conversions|ToFloat(Integer) (LocalVariables|GetY))) (Grid|GetTileCost "NewEnumerator4") 0 0 0 "(X=0.000000,Y=0.000000)")))))))

(fn SpawnTile
  (params (bSoawnNoneTile :type Boolean))
  (bind _struct_tile (Variables|Grid|Getstruct_Tile))
  (bind _keys (Utilities|Map|Keys (Variables|Grid|Getstruct_Tile)))
  (for _array_element _keys
    (if (or (Utilities|Enum|NotEqual(Enum) (.groundtype (.Value (Utilities|Map|Find _struct_tile _array_element))) "NewEnumerator4") bSoawnNoneTile)
      (bind _returnvalue (Game|SpawnActorfromClass "/Game/Blueprints/Grids/BP_GridTIle.BP_GridTIle_C" (Math|Conversions|ToTransform(Vector) (.worldlocation (.Value (Utilities|Map|Find _struct_tile _array_element)))) "Undefined" 0 0))
      (Variables|/Game/Blueprints/Grids/BP_GridTIle.BP_GridTIle_C|SetgridIndex _returnvalue _array_element)
      (Variables|/Game/Blueprints/Grids/BP_GridTIle.BP_GridTIle_C|Setbp_Grid _returnvalue self)
      (Utilities|Map|Add _struct_tile _array_element (Utilities|Struct|MakeStruct_Tiles 0 (.groundtype (.Value (Utilities|Map|Find _struct_tile _array_element))) (.worldlocation (.Value (Utilities|Map|Find _struct_tile _array_element))) (.gridindex (.Value (Utilities|Map|Find _struct_tile _array_element))) (.tilecost (.Value (Utilities|Map|Find _struct_tile _array_element))) (.finalcost (.Value (Utilities|Map|Find _struct_tile _array_element))) (.costfromstart (.Value (Utilities|Map|Find _struct_tile _array_element))) (.estimatedcosttotarget (.Value (Utilities|Map|Find _struct_tile _array_element))) (.previoustile (.Value (Utilities|Map|Find _struct_tile _array_element))))))))

(fn GetTileCost
  (params (grindIndex :type Enum_GroundTypes%20Enum :default "NewEnumerator0"))
  (switch Utilities|FlowControl|Switch|SwitchonEnum_GroundTypes grindIndex
    (:NewEnumerator0
      (LocalVariables|SetCost 1))
    (:NewEnumerator1
      (LocalVariables|SetCost 2))
    (:NewEnumerator2
      (LocalVariables|SetCost 5))
    (:NewEnumerator3
      (LocalVariables|SetCost 999 :!label _label))
    (:NewEnumerator4
      (goto _label)))
  (return (LocalVariables|GetCost)))

(fn GetTileNeighbours
  (params (gridIndex :type Vector%202D%20Structure))
  (bind _output_get (LocalVariables|SetpossivleNeighbours (Utilities|Array|MakeArray "(X=1.000000,Y=0.000000)" "(X=0.000000,Y=1.000000)" "(X=-1.000000,Y=0.000000)" "(X=0.000000,Y=-1.000000)")))
  (for _array_element _output_get
    (if (.ReturnValue (Utilities|Map|Find (Variables|Grid|Getstruct_Tile) (+ _array_element gridIndex)))
      (if (and (Utilities|Enum|NotEqual(Enum) (.groundtype (.Value (Utilities|Map|Find (Variables|Grid|Getstruct_Tile) (+ _array_element gridIndex)))) "NewEnumerator4") (Utilities|Enum|NotEqual(Enum) (.groundtype (.Value (Utilities|Map|Find (Variables|Grid|Getstruct_Tile) (+ _array_element gridIndex)))) "NewEnumerator3"))
        (Utilities|Array|AddUnique (LocalVariables|GetoutNeighbours) (+ _array_element gridIndex)))))
  (return (LocalVariables|GetoutNeighbours)))

(fn GetEstimatedCosttoTarget
  (params (currentTile :type Vector%202D%20Structure) (targetTile :type Vector%202D%20Structure))
  (bind _returnvalue (- currentTile targetTile))
  (return (Math|Float|Round (+ (Math|Float|Absolute(Float) (.x _returnvalue)) (Math|Float|Absolute(Float) (.y _returnvalue))))))

(fn FindPathtoTarget
  (params (startTile :type Vector%202D%20Structure) (targetTile :type Vector%202D%20Structure))
  (bind _struct_tile (Variables|Grid|Getstruct_Tile))
  (bind _struct_tile_2 (Variables|Grid|Getstruct_Tile))
  (bind _struct_tile_3 (Variables|Grid|Getstruct_Tile))
  (bind _struct_tile_4 (Variables|Grid|Getstruct_Tile))
  (LocalVariables|SetstartTileL startTile)
  (LocalVariables|SettargetTileL targetTile)
  (if (Math|Boolean|ANDBoolean (.ReturnValue (Utilities|Map|Find (Variables|Grid|Getstruct_Tile) (LocalVariables|GettargetTileL))) (Utilities|Enum|NotEqual(Enum) (.groundtype (.Value (Utilities|Map|Find (Variables|Grid|Getstruct_Tile) (LocalVariables|GettargetTileL)))) "NewEnumerator4") (Utilities|Enum|NotEqual(Enum) (.groundtype (.Value (Utilities|Map|Find (Variables|Grid|Getstruct_Tile) (LocalVariables|GettargetTileL)))) "NewEnumerator3"))
    (Utilities|FlowControl|Sequence
      (:then_0
        ;[1 1 1] Default Values
        (bind _keys (Utilities|Map|Keys (Variables|Grid|Getstruct_Tile)))
        (for _array_element _keys
          (Utilities|Map|Add _struct_tile_4 _array_element (Utilities|Struct|MakeStruct_Tiles (.tileactor (.Value (Utilities|Map|Find _struct_tile_4 _array_element))) (.groundtype (.Value (Utilities|Map|Find _struct_tile_4 _array_element))) (.worldlocation (.Value (Utilities|Map|Find _struct_tile_4 _array_element))) (.gridindex (.Value (Utilities|Map|Find _struct_tile_4 _array_element))) (.tilecost (.Value (Utilities|Map|Find _struct_tile_4 _array_element))) 999 999 999 "(X=0.000000,Y=0.000000)")))
        (Utilities|Map|Add _struct_tile_2 (LocalVariables|GetstartTileL) (Utilities|Struct|MakeStruct_Tiles (.tileactor (.Value (Utilities|Map|Find _struct_tile_2 (LocalVariables|GetstartTileL)))) (.groundtype (.Value (Utilities|Map|Find _struct_tile_2 (LocalVariables|GetstartTileL)))) (.worldlocation (.Value (Utilities|Map|Find _struct_tile_2 (LocalVariables|GetstartTileL)))) (.gridindex (.Value (Utilities|Map|Find _struct_tile_2 (LocalVariables|GetstartTileL)))) (.tilecost (.Value (Utilities|Map|Find _struct_tile_2 (LocalVariables|GetstartTileL)))) (Pathfinding|GetEstimatedCosttoTarget (LocalVariables|GetstartTileL) (LocalVariables|GettargetTileL)) 0 (Pathfinding|GetEstimatedCosttoTarget (LocalVariables|GetstartTileL) (LocalVariables|GettargetTileL)) "(X=0.000000,Y=0.000000)")))
      (:then_1
        (LocalVariables|SetcurrentTile (LocalVariables|GetstartTileL))
        (Utilities|Array|AddUnique (LocalVariables|GetopenSet) (LocalVariables|GetstartTileL))
        (while (> (Utilities|Array|Length (LocalVariables|GetopenSet)) 0)
          (LocalVariables|SetopenSetCheapest (Utilities|Array|Get(acopy) (LocalVariables|GetopenSet)))
          (for _array_element_2 (LocalVariables|GetopenSet)
            (if (< (.finalcost (.Value (Utilities|Map|Find _struct_tile _array_element_2))) (.finalcost (.Value (Utilities|Map|Find _struct_tile (LocalVariables|GetopenSetCheapest)))))
              (LocalVariables|SetopenSetCheapest _array_element_2 :!label _label)
              (elif (== (.finalcost (.Value (Utilities|Map|Find _struct_tile _array_element_2))) (.finalcost (.Value (Utilities|Map|Find _struct_tile (LocalVariables|GetopenSetCheapest)))))
                (if (< (.estimatedcosttotarget (.Value (Utilities|Map|Find _struct_tile _array_element_2))) (.estimatedcosttotarget (.Value (Utilities|Map|Find _struct_tile (LocalVariables|GetopenSetCheapest)))))
                  (goto _label)))))
          (LocalVariables|SetcurrentTile (LocalVariables|GetopenSetCheapest))
          (Utilities|Array|RemoveItem (LocalVariables|GetopenSet) (LocalVariables|GetcurrentTile))
          (Utilities|Array|AddUnique (LocalVariables|GetclosedSet) (LocalVariables|GetcurrentTile))
          (for _array_element_3 (Pathfinding|GetTileNeighbours (LocalVariables|GetcurrentTile))
            (LocalVariables|SetcurrentNeighbour _array_element_3)
            (if (not (Utilities|Array|ContainsItem (LocalVariables|GetclosedSet) (LocalVariables|GetcurrentNeighbour)))
              (LocalVariables|SetcurrentNeighbourCostFromStart (+ (.costfromstart (.Value (Utilities|Map|Find (Variables|Grid|Getstruct_Tile) (LocalVariables|GetcurrentTile)))) (.tilecost (.Value (Utilities|Map|Find (Variables|Grid|Getstruct_Tile) (LocalVariables|GetcurrentNeighbour))))))
              (if (not (Utilities|Array|ContainsItem (LocalVariables|GetopenSet) (LocalVariables|GetcurrentNeighbour)))
                (Utilities|Array|AddUnique (LocalVariables|GetopenSet) (LocalVariables|GetcurrentNeighbour))
                (Utilities|Map|Add _struct_tile_3 (LocalVariables|GetcurrentNeighbour) (Utilities|Struct|MakeStruct_Tiles (.tileactor (.Value (Utilities|Map|Find _struct_tile_3 (LocalVariables|GetcurrentNeighbour)))) (.groundtype (.Value (Utilities|Map|Find _struct_tile_3 (LocalVariables|GetcurrentNeighbour)))) (.worldlocation (.Value (Utilities|Map|Find _struct_tile_3 (LocalVariables|GetcurrentNeighbour)))) (.gridindex (.Value (Utilities|Map|Find _struct_tile_3 (LocalVariables|GetcurrentNeighbour)))) (.tilecost (.Value (Utilities|Map|Find _struct_tile_3 (LocalVariables|GetcurrentNeighbour)))) (+ (LocalVariables|GetcurrentNeighbourCostFromStart) (Pathfinding|GetEstimatedCosttoTarget (LocalVariables|GetcurrentNeighbour) (LocalVariables|GettargetTileL))) (LocalVariables|GetcurrentNeighbourCostFromStart) (Pathfinding|GetEstimatedCosttoTarget (LocalVariables|GetcurrentNeighbour) (LocalVariables|GettargetTileL)) (LocalVariables|GetcurrentTile)) :!label _label_2)
                (if (Math|Vector|Equal(Vector) (LocalVariables|GetcurrentNeighbour) (LocalVariables|GettargetTileL) 0.0001)
                  (Variables|Default|Setpath (Pathfinding|RetracePath (LocalVariables|GettargetTileL) (LocalVariables|GetstartTileL)))
                  (return))
                (elif (< (LocalVariables|GetcurrentNeighbourCostFromStart) (.costfromstart (.Value (Utilities|Map|Find _struct_tile_3 (LocalVariables|GetcurrentNeighbour)))))
                  (goto _label_2))))))
        ;[1 1 1] Fail
        (return)))))

(fn RetracePath
  (params (targetTile :type Vector%202D%20Structure) (startTile :type Vector%202D%20Structure))
  (LocalVariables|SetcurrentTile targetTile)
  (while (Math|Vector|NotEqual(Vector) (LocalVariables|GetcurrentTile) startTile 0.0001)
    (Utilities|Array|AddUnique (LocalVariables|GetinvertedPath) (LocalVariables|GetcurrentTile))
    (LocalVariables|SetcurrentTile (.previoustile (.Value (Utilities|Map|Find (Variables|Grid|Getstruct_Tile) (LocalVariables|GetcurrentTile))))))
  (bind _arrayelement (Utilities|Array|ReverseforEachLoop (LocalVariables|GetinvertedPath))
    (:LoopBody
      (Utilities|Array|AddUnique (LocalVariables|GetoutPath) _arrayelement))
    (:Completed
      (return (LocalVariables|GetoutPath)))))

(fn HighlightCurrentPath
  (params (bIsForHighlight :type Boolean))
  (for _array_element (Variables|Default|Getpath)
    (Utilities|IsValid (.tileactor (.Value (Utilities|Map|Find (Variables|Grid|Getstruct_Tile) _array_element)))
      (:Is%20Valid
        (Default|EventIsinPath (Variables|BP_Grid_C|GetoveredTile (.tileactor (.Value (Utilities|Map|Find (Variables|Grid|Getstruct_Tile) _array_element)))) bIsForHighlight)))))