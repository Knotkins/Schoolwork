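; BP_GridTIle is a single clickable tile of a BpGrid, showing ground type and hover, selection and path states.
; On BeginPlay, after a short delay, it colours itself, scales to the grid's TileSize and passes grid and index to its W_GridTile widget.
; Hover and click set local flags and notify the grid; cursor exit is empty.
; Material parameters show selection and a colour from the grid's tile data, brightened on hover, black on paths.
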(event OnBeginCursorOver(StaticMesh)
  (params (TouchedComponent :type Primitive%20Component%20Object%20Reference))
  (CallFunction|EventStartOverTIle)
  (Default|EventNewTileOvered (Variables|Grid|Getbp_Grid) self))

(event OnEndCursorOver(StaticMesh)
  (params (TouchedComponent :type Primitive%20Component%20Object%20Reference)))

(event OnClicked(StaticMesh)
  (params (TouchedComponent :type Primitive%20Component%20Object%20Reference) (ButtonPressed :type Key%20Structure :default "None"))
  (CallFunction|EventSelectTile)
  (Default|EventNewTileSelected (Variables|Grid|Getbp_Grid) self))

(event Custom|Event_DeselectTIle
  (Variables|Grid|SetbIsSelect false)
  (Grid|SetTIleColour))

(event Custom|Event_SelectTile
  (Variables|Grid|SetbIsSelect true)
  (Grid|SetTIleColour))

(event Custom|Event_EndOverTile
  (Variables|Grid|SetbIsOvered false)
  (Grid|SetTIleColour))

(event Custom|Event_StartOverTIle
  (Variables|Grid|SetbIsOvered true)
  (Grid|SetTIleColour))

(event Custom|Event_IsInPath
  (params (bIsInPath :type Boolean))
  (Variables|Default|SetbIsInPath bIsInPath)
  (Grid|SetTIleColour))

(event EventBeginPlay
  (Utilities|FlowControl|Delay 0.2)
  (Grid|SetTIleColour)
  (Grid|SetTileSize)
  (Debug|SetWidgetVariables))

(fn ConstructionScript)

(fn SetTileSize
  (bind _bp_grid (Variables|Grid|Getbp_Grid))
  (bind _staticmesh (Variables|Default|GetStaticMesh))
  (bind _returnvalue (Transformation|GetWorldScale _staticmesh))
  (bind _tilesize (Variables|/Game/Blueprints/Grids/BP_Grid.BP_Grid_C|GetTileSize _bp_grid))
  (bind _returnvalue_2 (/ _tilesize 5e+01))
  (bind _returnvalue_3 (Math|Conversions|ToVector(Float) _returnvalue_2))
  (bind _returnvalue_4 (* _returnvalue _returnvalue_3))
  (Transformation|SetWorldScale3D _staticmesh (Math|Vector|MakeVector (.x _returnvalue_4) (.y _returnvalue_4) 1.0)))

(fn SetTIleColour
  (Utilities|FlowControl|Sequence
    (:then_0
      (switch Utilities|FlowControl|Switch|SwitchonEnum_GroundTypes (.groundtype (Grid|GetTIleData))
        (:NewEnumerator0
          (LocalVariables|SetTileColour "(R=0.000000,G=1.000000,B=0.085310,A=1.000000)"))
        (:NewEnumerator1
          (LocalVariables|SetTileColour "(R=0.869792,G=0.855820,B=0.000000,A=1.000000)"))
        (:NewEnumerator2
          (LocalVariables|SetTileColour "(R=0.817708,G=0.275223,B=0.001199,A=1.000000)"))
        (:NewEnumerator3
          (LocalVariables|SetTileColour "(R=0.598958,G=0.000000,B=0.000000,A=1.000000)"))
        (:NewEnumerator4
          (LocalVariables|SetTileColour "(R=0.057292,G=0.047147,B=0.047147,A=1.000000)"))))
    (:then_1
      (if (Variables|Grid|GetbIsSelect)
        (Rendering|Material|SetScalarParameterValueonMaterials (Variables|Default|GetStaticMesh) "blsSelected" 1.0)
        (else
          (Rendering|Material|SetScalarParameterValueonMaterials (Variables|Default|GetStaticMesh) "blsSelected" 0.0))))
    (:then_2
      (if (Variables|Grid|GetbIsOvered)
        (LocalVariables|SettileColour (Math|Conversions|ToLinearColor(Vector) (+ (Math|Conversions|ToVector(LinearColor) (LocalVariables|GettileColour)) 3.0)))))
    (:then_3
      (if (Variables|Default|GetbIsInPath)
        (LocalVariables|SettileColour "")))
    (:then_4
      (Rendering|Material|SetVectorParameterValueonMaterials (Variables|Default|GetStaticMesh) "TileColour" (Math|Conversions|ToVector(LinearColor) (LocalVariables|GettileColour))))))

(fn GetTIleData
  (return (.Value (Utilities|Map|Find (Variables|/Game/Blueprints/Grids/BP_Grid.BP_Grid_C|Getstruct_Tile (Variables|Grid|Getbp_Grid)) (Variables|Grid|GetgridIndex)))))

(fn SetWidgetVariables
  (bind _asw_grid_tile (Utilities|Casting|CastToW_GridTile (UserInterface|GetUserWidgetObject (Variables|Default|GetWidget))))
  (Variables|/Game/Blueprints/Grids/W_GridTile.W_GridTile_C|Setgrid _asw_grid_tile (Variables|Grid|Getbp_Grid))
  (Variables|/Game/Blueprints/Grids/W_GridTile.W_GridTile_C|SetgridIdex _asw_grid_tile (Variables|Grid|GetgridIndex)))